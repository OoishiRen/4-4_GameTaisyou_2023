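; BP_Enemy_Paturn picks an enemy's next command from preset two-turn patterns.
; Enemy_Paturn takes a Selection to choose one of three patterns, then uses EnemyTurn to pick that step's command number.
; SetEnemyPaturn writes it into the EnemyA or EnemyB struct on BP_One_v_One_GameInstance, based on EnemyName.
; EnemyTurn advances per call; after two steps it resets and clears the SetPaturn flag.
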(event `Enemy_Paturn`
  (params (Selection :type Integer) (EnemyName :type Name))
  (set `self.SetPaturn` true)
  (switch `int` Selection
    (:`0`
      (switch `int` (`self.EnemyTurn`)
        (:`0`
          (`self.Set_Enemy_Paturn` EnemyName))
        (:`1`
          (`self.Set_Enemy_Paturn` EnemyName 1))))
    (:`1`
      (switch `int` (`self.EnemyTurn`)
        (:`0`
          (`self.Set_Enemy_Paturn` EnemyName 1))
        (:`1`
          (`self.Set_Enemy_Paturn` EnemyName 1))))
    (:`2`
      (switch `int` (`self.EnemyTurn`)
        (:`0`
          (`self.Set_Enemy_Paturn` EnemyName))
        (:`1`
          (`self.Set_Enemy_Paturn` EnemyName 2))))))

(fn `Set_Enemy_Paturn`
  (params (EnemyName :type Name) (ComandNum :type Integer))
  (bind _enemyturn (`self.EnemyTurn`))
  (bind _asbp_one_v_one_game_instance (cast `/Game/BP/BP_One_v_One_GameInstance` (`GameplayStatics.GetGameInstance`) :!pure true))
  (if (== EnemyName "EnemyA")
    (bind _structout (setmembers `/Game/BP/BP_Character` :`StructRef` (`/Game/BP/BP_One_v_One_GameInstance.Enemy_A` _asbp_one_v_one_game_instance) :`ComandNum` ComandNum))
    (set `/Game/BP/BP_One_v_One_GameInstance.Enemy_A` _structout _asbp_one_v_one_game_instance)
    (else
      (bind _structout_2 (setmembers `/Game/BP/BP_Character` :`StructRef` (`/Game/BP/BP_One_v_One_GameInstance.Enemy_B` _asbp_one_v_one_game_instance) :`ComandNum` ComandNum))
      (set `/Game/BP/BP_One_v_One_GameInstance.Enemy_B` _structout_2 _asbp_one_v_one_game_instance)))
  (`/Engine/EditorBlueprintResources/StandardMacros.IncrementInt` _enemyturn
    (:`  `
      (if (>= _enemyturn 2)
        (set `self.SetPaturn` false)
        (set `self.EnemyTurn` 0)))))

(fn `UserConstructionScript`)