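; Game instance for a turn-based RPG battle that holds the shared combat data for a Hero and two enemies.
; Setup functions fill character stats, per-character special attack lists and five player items with healing, damage and buff values, and make EnemyA the initial target.
; Result reads the Dead flags and sets the win, lose and result flags, requiring both enemies dead to win.
; The combined item array node is unconnected.
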(fn `Create_Character`
  (set `self.Hero` (make `/Game/BP/BP_Character` "Hero" 300 300 50 50 300 300 30 30 10 10))
  (bind _output_get (set `self.Enemy_A` (make `/Game/BP/BP_Character` "Enemy" 200 200 50 50 18 18 28 28 10 10 1.0 true)))
  (set `self.Target` _output_get)
  (set `self.Enemy_B` (make `/Game/BP/BP_Character` "Enemy2" 300 300 100 100 28 28 15 15 15 15 1.0 true)))

(fn `Enemy1_Special`
  (set `self.Enemy_Spe` (`|MakeArray` (make `/Game/BP/BP_SpecialAtk` "フレイム" 10 20 1.0 20) (make `/Game/BP/BP_SpecialAtk` "ためる" 5 0 2.0 30 1.0 0 1.0 0 1.0 true) (make `/Game/BP/BP_SpecialAtk` "きりつける" 5 50 1.0 20) (make `/Game/BP/BP_SpecialAtk` "きゅうしょづき" 15 50 1.0 15))))

(fn `Enemy2_Special`
  (set `self.Enemy2_Spe` (`|MakeArray` (make `/Game/BP/BP_SpecialAtk` "メガフレイム" 10 50 1.0 20) (make `/Game/BP/BP_SpecialAtk` "ためる" 5 0 2.0 30 1.0 0 1.0 0 1.0 true) (make `/Game/BP/BP_SpecialAtk` "きりつける" 5 42 1.0 15) (make `/Game/BP/BP_SpecialAtk` "きゅうしょづき" 15 52 1.0 10) (make `/Game/BP/BP_SpecialAtk` "いやす" 30 0 1.0 30 1.0 0 1.0 60 1.0 false false true))))

(fn `Player_Item`
  (set `self.Player_Item_1` (make `/Game/BP/BP_ItemName` 3 3 "モロトフ" 30 0 0 1.0 20))
  (set `self.Player_Item_2` (make `/Game/BP/BP_ItemName` 5 5 "回復薬" 0 60 0 1.0 999 1.0 false false true))
  (set `self.Player_Item_3` (make `/Game/BP/BP_ItemName` 2 2 "魔力回復薬" 0 0 25 1.0 999 1.0 false false true))
  (set `self.Player_Item_4` (make `/Game/BP/BP_ItemName` 1 1 "力の丸薬" 0 0 0 2.0 999 1.0 false false false 3))
  (set `self.Player_Item_5` (make `/Game/BP/BP_ItemName` 1 1 "鎮痛剤" 0 10 0 1.0 999 1.5 false false false 0 3)))

(fn `Player_Special`
  (set `self.Player_Spe` (`|MakeArray` (make `/Game/BP/BP_SpecialAtk` "フレイム" 10 30 1.0 20) (make `/Game/BP/BP_SpecialAtk` "ためる" 5 0 2.0 30 1.0 0 1.0 0 1.0 true) (make `/Game/BP/BP_SpecialAtk` "きりつける" 5 30 1.0 20) (make `/Game/BP/BP_SpecialAtk` "いやす" 10 0 1.0 20 1.0 0 1.0 40 1.0 false false true) (make `/Game/BP/BP_SpecialAtk` "きゅうしょづき" 15 45 1.0 20))))

(fn `Result`
  (if (`.Dead_32_2DD09B514FB38163D3DCB285D46251D5` (break `/Game/BP/BP_Character` (`self.Hero`)))
    (set `self.Player_Win` false)
    (set `self.Player_Lose` true)
    (set `self.ResultFlg` true)
    (elif (and (`.Dead_32_2DD09B514FB38163D3DCB285D46251D5` (break `/Game/BP/BP_Character` (`self.Enemy_A`))) (`.Dead_32_2DD09B514FB38163D3DCB285D46251D5` (break `/Game/BP/BP_Character` (`self.Enemy_B`))))
      (set `self.Player_Lose` false)
      (set `self.Player_Win` true)
      (set `self.ResultFlg` true)
      (else
        (set `self.Player_Win` false) ; どっちも残っていた場合
        (set `self.Player_Lose` false)
        (set `self.ResultFlg` false)))))