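; BP_Item applies battle item effects to character structs and writes the results to BP_One_v_One_GameInstance.
; Use_ITem picks heal, attack buff, defence buff or damage from a passed item struct's fields, after checking quantity.
; Use_Item2 switches on slot index for molotov, HP potion, MP potion, attack pill and painkiller, decrementing stock.
; Healing clamps at maximum, full HP/MP only sets a flag, and molotov hits also update EnemyA or EnemyB.
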(event `Use_ITem`
  (params (Player :type "/Game/BP/BP_Character Structure (by ref)") (TargetEnemy :type "/Game/BP/BP_Character Structure (by ref)") (BP_ItemName :type "/Game/BP/BP_ItemName Structure (by ref)"))
  (bind (_charactername _maxhp _nowhp _maxmp _nowmp _defultatk _nowatk _defultspd _nowspd _defultdef _nowdef) (break `/Game/BP/BP_Character` TargetEnemy))
  (bind (_default_quantity _now_quantity _itemname _atk _healhp _healmp _atkbuf _spd _defencebuf _atk_buf _defbuf _healbuf) (break `/Game/BP/BP_ItemName` BP_ItemName))
  (bind _returnvalue (+ _healhp _nowhp))
  (bind _returnvalue_2 (+ _healmp _nowmp))
  (bind _asbp_one_v_one_game_instance (cast `/Game/BP/BP_One_v_One_GameInstance` (`GameplayStatics.GetGameInstance`) :!pure true))
  (bind _asbp_one_v_one_game_instance_2 (cast `/Game/BP/BP_One_v_One_GameInstance` (`GameplayStatics.GetGameInstance`) :!pure true))
  (if (> _now_quantity 0)
    (if _healbuf
      (if (or (>= _returnvalue _maxhp) (>= _returnvalue_2 _maxmp))
        (bind _structout (setmembers `/Game/BP/BP_Character` :`StructRef` Player :`NowHP` _maxhp :`NowMP` _maxmp :`NowSpd` _spd)) ; 超えてたらデフォルト数値にする
        (set `/Game/BP/BP_One_v_One_GameInstance.Hero` _structout _asbp_one_v_one_game_instance)
        (else
          (bind _structout_2 (setmembers `/Game/BP/BP_Character` :`StructRef` Player :`NowHP` _returnvalue :`NowMP` _returnvalue_2 :`NowSpd` _spd)) ; 回復した後の数値入れる
          (set `/Game/BP/BP_One_v_One_GameInstance.Hero` _structout_2 _asbp_one_v_one_game_instance)))
      (elif _atk_buf
        (bind _structout_3 (setmembers `/Game/BP/BP_Character` :`StructRef` Player :`NowAtk` (`KismetMathLibrary.FTrunc` (* _nowatk _atkbuf)) :`NowSpd` _spd)) ; 攻撃バフ後の数値
        (set `/Game/BP/BP_One_v_One_GameInstance.Hero` _structout_3 _asbp_one_v_one_game_instance)
        (elif _defbuf
          (bind _structout_4 (setmembers `/Game/BP/BP_Character` :`StructRef` Player :`NowSpd` _spd :`NowDef` (`KismetMathLibrary.FTrunc` (* _nowdef _defencebuf)))) ; 防御バフ後の数値
          (set `/Game/BP/BP_One_v_One_GameInstance.Hero` _structout_4 _asbp_one_v_one_game_instance)
          (else
            (bind _structout_5 (setmembers `/Game/BP/BP_Character` :`StructRef` TargetEnemy :`NowHP` (- _nowhp _atk) :`NowSpd` _spd :`Damage` _atk)) ; ここら辺からダメージ処理入る
            (set `/Game/BP/BP_One_v_One_GameInstance.Target` _structout_5 _asbp_one_v_one_game_instance_2)
            (bind _structout_6 (setmembers `/Game/BP/BP_ItemName` :`StructRef` BP_ItemName :`Now_Quantity` (- (`.Now_Quantity_58_387752974356BE832F52E68B049F8B07` (break `/Game/BP/BP_ItemName` BP_ItemName)) 1)))
            (set `/Game/BP/BP_One_v_One_GameInstance.Player_Ite` (`|MakeArray` _structout_6 _structout_6 _structout_6 _structout_6 _structout_6) _asbp_one_v_one_game_instance_2)
            (if (<= (`.NowHP_22_7C1D8F80417BE5B3F6BAC29D355D5182` (break `/Game/BP/BP_Character` TargetEnemy)) 0)
              (bind _structout_7 (setmembers `/Game/BP/BP_Character` :`StructRef` TargetEnemy :`Dead` true))
              (set `/Game/BP/BP_One_v_One_GameInstance.Target` _structout_7 _asbp_one_v_one_game_instance_2))))))))

(event `Use_Item2`
  (params (TargetEnemy :type "/Game/BP/BP_Character Structure (by ref)") (Player :type "/Game/BP/BP_Character Structure") (ItemNum :type Integer))
  (bind ((`MaxHP_19_CA06E95947FC7016BD1C69AC8C5500BD` _maxhp)) (break `/Game/BP/BP_Character` Player))
  (bind ((`MaxMP_24_A1416E0E43116919C65C4BB31DA5B979` _maxmp)) (break `/Game/BP/BP_Character` Player))
  (bind ((`MaxMP_24_A1416E0E43116919C65C4BB31DA5B979` _maxmp_2) (`NowMP_26_765052624FE1436EC2219F8D360B25BA` _nowmp)) (break `/Game/BP/BP_Character` Player))
  (bind ((`MaxHP_19_CA06E95947FC7016BD1C69AC8C5500BD` _maxhp_2) (`NowHP_22_7C1D8F80417BE5B3F6BAC29D355D5182` _nowhp)) (break `/Game/BP/BP_Character` Player))
  (bind ((`NowHP_22_7C1D8F80417BE5B3F6BAC29D355D5182` _nowhp_2) (`NowMP_26_765052624FE1436EC2219F8D360B25BA` _nowmp_2) (`NowDef_42_7491192F427A3681A29158AE6392073B` _nowdef)) (break `/Game/BP/BP_Character` Player))
  (bind ((`NowHP_22_7C1D8F80417BE5B3F6BAC29D355D5182` _nowhp_3)) (break `/Game/BP/BP_Character` TargetEnemy))
  (bind _asbp_one_v_one_game_instance (`self.Cast_To_GameInstance`))
  (bind _asbp_one_v_one_game_instance_2 (`self.Cast_To_GameInstance`))
  (bind _asbp_one_v_one_game_instance_3 (`self.Cast_To_GameInstance`))
  (bind _asbp_one_v_one_game_instance_4 (`self.Cast_To_GameInstance`))
  (bind _asbp_one_v_one_game_instance_5 (`self.Cast_To_GameInstance`))
  (bind _player_item_1 (`/Game/BP/BP_One_v_One_GameInstance.Player_Item_1` (`self.Cast_To_GameInstance`)))
  (bind ((`Now_Quantity_58_387752974356BE832F52E68B049F8B07` _now_quantity) (`HealMP_42_D6C7A4654BCB880703A22593AD22B2AA` _healmp)) (break `/Game/BP/BP_ItemName` (`/Game/BP/BP_One_v_One_GameInstance.Player_Item_3` (`self.Cast_To_GameInstance`))))
  (bind ((`Now_Quantity_58_387752974356BE832F52E68B049F8B07` _now_quantity_2) (`HealHP_43_A92F38C142DA32203FA90FA6A5E90B72` _healhp)) (break `/Game/BP/BP_ItemName` (`/Game/BP/BP_One_v_One_GameInstance.Player_Item_2` (`self.Cast_To_GameInstance`))))
  (bind ((`Now_Quantity_58_387752974356BE832F52E68B049F8B07` _now_quantity_3) (`DefenceBuf_35_5C82CF344410FC97AA52F48BCAB5E5D0` _defencebuf)) (break `/Game/BP/BP_ItemName` (`/Game/BP/BP_One_v_One_GameInstance.Player_Item_5` (`self.Cast_To_GameInstance`))))
  (bind ((`Now_Quantity_58_387752974356BE832F52E68B049F8B07` _now_quantity_4) (`Atk_5_5004DF4447DE3C6063662EBC66F977F8` _atk)) (break `/Game/BP/BP_ItemName` _player_item_1))
  (bind _returnvalue (+ _healhp _nowhp_2))
  (bind _returnvalue_2 (+ _healmp _nowmp_2))
  (switch `int` ItemNum
    (:`0`
      (bind _structout (setmembers `/Game/BP/BP_Character` :`StructRef` TargetEnemy :`NowHP` (- _nowhp_3 _atk) :`Damage` _atk)) ; 敵の情報
      (set `/Game/BP/BP_One_v_One_GameInstance.Target` _structout (`self.Cast_To_GameInstance`))
      (if (== (`.CharacterName_4_60DFF35B41F76AE7F168749DF3E39C61` (break `/Game/BP/BP_Character` TargetEnemy)) "Enemy")
        (set `/Game/BP/BP_One_v_One_GameInstance.Enemy_A` _structout _asbp_one_v_one_game_instance_4)
        (else
          (set `/Game/BP/BP_One_v_One_GameInstance.Enemy_B` _structout _asbp_one_v_one_game_instance_4)))
      (bind _structout_2 (setmembers `/Game/BP/BP_ItemName` :`StructRef` _player_item_1 :`Now_Quantity` (- _now_quantity_4 1))) ; アイテム１号（モロトフ）
      (set `/Game/BP/BP_One_v_One_GameInstance.Player_Item_1` _structout_2 (`self.Cast_To_GameInstance`))
      (if (<= _nowhp_3 0)
        (bind _structout_3 (setmembers `/Game/BP/BP_Character` :`StructRef` TargetEnemy :`Dead` true)) ; 敵の情報
        (set `/Game/BP/BP_One_v_One_GameInstance.Target` _structout_3 (`self.Cast_To_GameInstance`))))
    (:`1`
      (if (== _maxhp_2 _nowhp)
        (set `/Game/BP/BP_One_v_One_GameInstance.HP_MAX` true _asbp_one_v_one_game_instance_3)
        (else
          (set `/Game/BP/BP_One_v_One_GameInstance.HP_MAX` false _asbp_one_v_one_game_instance_3)
          (if (>= _returnvalue _maxhp)
            (bind _structout_4 (setmembers `/Game/BP/BP_Character` :`StructRef` Player :`NowHP` _maxhp)) ; プレイヤーの情報
            (set `/Game/BP/BP_One_v_One_GameInstance.Hero` _structout_4 _asbp_one_v_one_game_instance_5)
            (else
              (bind _structout_5 (setmembers `/Game/BP/BP_Character` :`StructRef` Player :`NowHP` _returnvalue)) ; プレイヤーの情報
              (set `/Game/BP/BP_One_v_One_GameInstance.Hero` _structout_5 _asbp_one_v_one_game_instance_5)))
          (bind _structout_6 (setmembers `/Game/BP/BP_ItemName` :`StructRef` (`/Game/BP/BP_One_v_One_GameInstance.Player_Item_2` (`self.Cast_To_GameInstance`)) :`Now_Quantity` (- _now_quantity_2 1))) ; アイテム２号（回復薬）
          (set `/Game/BP/BP_One_v_One_GameInstance.Player_Item_2` _structout_6 (`self.Cast_To_GameInstance`)))))
    (:`2`
      (if (== _maxmp_2 _nowmp)
        (set `/Game/BP/BP_One_v_One_GameInstance.MP_MAX` true _asbp_one_v_one_game_instance_2)
        (else
          (set `/Game/BP/BP_One_v_One_GameInstance.MP_MAX` false _asbp_one_v_one_game_instance_2)
          (if (>= _returnvalue_2 _maxmp)
            (bind _structout_7 (setmembers `/Game/BP/BP_Character` :`StructRef` Player :`NowMP` _maxmp)) ; プレイヤーの情報
            (set `/Game/BP/BP_One_v_One_GameInstance.Hero` _structout_7 _asbp_one_v_one_game_instance)
            (else
              (bind _structout_8 (setmembers `/Game/BP/BP_Character` :`StructRef` Player :`NowMP` _returnvalue_2)) ; プレイヤーの情報
              (set `/Game/BP/BP_One_v_One_GameInstance.Hero` _structout_8 _asbp_one_v_one_game_instance)))
          (bind _structout_9 (setmembers `/Game/BP/BP_ItemName` :`StructRef` (`/Game/BP/BP_One_v_One_GameInstance.Player_Item_3` (`self.Cast_To_GameInstance`)) :`Now_Quantity` (- _now_quantity 1))) ; アイテム３号（魔力回復薬）
          (set `/Game/BP/BP_One_v_One_GameInstance.Player_Item_3` _structout_9 (`self.Cast_To_GameInstance`)))))
    (:`3`
      (`self.Atack_Buf_Item` Player))
    (:`4`
      (bind _structout_10 (setmembers `/Game/BP/BP_Character` :`StructRef` Player :`NowDef` (`KismetMathLibrary.FTrunc` (* _nowdef _defencebuf)))) ; プレイヤーの情報
      (set `/Game/BP/BP_One_v_One_GameInstance.Hero` _structout_10 (`self.Cast_To_GameInstance`))
      (bind _structout_11 (setmembers `/Game/BP/BP_ItemName` :`StructRef` (`/Game/BP/BP_One_v_One_GameInstance.Player_Item_5` (`self.Cast_To_GameInstance`)) :`Now_Quantity` (- _now_quantity_3 1))) ; アイテム５号（鎮痛剤）
      (set `/Game/BP/BP_One_v_One_GameInstance.Player_Item_5` _structout_11 (`self.Cast_To_GameInstance`)))))

(event `Atack_Buf_Item`
  (params (Player :type "/Game/BP/BP_Character Structure (by ref)"))
  (bind ((`Now_Quantity_58_387752974356BE832F52E68B049F8B07` _now_quantity) (`AtkBuf_33_E191D23944BF193DA2C73B8A1E89D5C6` _atkbuf)) (break `/Game/BP/BP_ItemName` (`/Game/BP/BP_One_v_One_GameInstance.Player_Item_4` (`self.Cast_To_GameInstance`))))
  (bind _structout (setmembers `/Game/BP/BP_Character` :`StructRef` Player :`NowAtk` (`KismetMathLibrary.FTrunc` (* (`.NowAtk_41_F1C25EFB436C26403D39C7B34EE08417` (break `/Game/BP/BP_Character` Player)) _atkbuf)))) ; プレイヤーの情報
  (set `/Game/BP/BP_One_v_One_GameInstance.Hero` _structout (`self.Cast_To_GameInstance`))
  (bind _structout_2 (setmembers `/Game/BP/BP_ItemName` :`StructRef` (`/Game/BP/BP_One_v_One_GameInstance.Player_Item_4` (`self.Cast_To_GameInstance`)) :`Now_Quantity` (- _now_quantity 1))) ; アイテム４号（力の丸薬）
  (set `/Game/BP/BP_One_v_One_GameInstance.Player_Item_4` _structout_2 (`self.Cast_To_GameInstance`)))

(fn `UserConstructionScript`)