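; BP_E1 is a battle enemy, apparently a dragon, that lunges to a fixed point and returns when BP_Battle flags an enemy attack.
; Tick polls that flag and uses Testflg to alternate between two Timeline-driven location lerps, attack and retreat.
; The attack plays a delayed, DoOnce-gated sound and spawns a hit effect at the GameInstance's player position.
; The retreat clears the battle flag and resets both timelines and the sound gate.
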(event `self.ReceiveTick`
  (params (DeltaSeconds :type "Float (single-precision)"))
  (if (`/Game/BP/BP_Battle.EnemyAttack` (cast `/Game/BP/BP_Battle` (`|GetArrayItem` (stale `self.ReceiveBeginPlay` _outactors)) :!pure true))
    (set `self.Soundflg` true)
    (if (`self.testflg`)
      (`self.Attack_Move`)
      (else
        (`self.Back_Move`)
        (`KismetSystemLibrary.Delay` 2.0)
        (set `self.testflg` true)))))

(event `self.ReceiveBeginPlay`
  (set `self.Default_Position` (`self.K2_GetActorLocation`))
  (bind _outactors (`GameplayStatics.GetAllActorsOfClass` "/Game/BP/BP_Battle.BP_Battle_C")))

(event `Attack_Move`
  (bind (_direction _enemy_move) (`Timeline|タイムライン_0`)
    (:`Update`
      (`self.K2_SetActorLocation` (`KismetMathLibrary.VLerp` (`self.Default_Position`) (-100.0 -90.0 300.0) _enemy_move))
      (if (`self.Soundflg`)
        (`KismetSystemLibrary.Delay` 0.25)
        (`/Engine/EditorBlueprintResources/StandardMacros.DoOnce` false :!label _label
          (:`Completed`
            (`GameplayStatics.PlaySound2D` "/Game/SE/Dragon_nomalAttack.Dragon_nomalAttack")
            (set `self.Soundflg` false)))))
    (:`Finished`
      (`GameplayStatics.SpawnEmitterAtLocation` "/Game/FX/P_Hit.P_Hit" (`/Game/BP/BP_One_v_One_GameInstance.PlayerPosition` (cast `/Game/BP/BP_One_v_One_GameInstance` (`GameplayStatics.GetGameInstance`) :!pure true)))
      (set `self.testflg` false))))

(event `Back_Move`
  (bind (_direction _enemy_move) (`Timeline|タイムライン_1`)
    (:`Update`
      (`self.K2_SetActorLocation` (`KismetMathLibrary.VLerp` (-100.0 -90.0 300.0) (`self.Default_Position`) _enemy_move)))
    (:`Finished`
      (set `/Game/BP/BP_Battle.EnemyAttack` false (cast `/Game/BP/BP_Battle` (`|GetArrayItem` (stale `self.ReceiveBeginPlay` _outactors)) :!pure true))
      (`TimelineComponent.SetNewTime` (`self.タイムライン_1`) 0.0)
      (`TimelineComponent.SetNewTime` (`self.タイムライン_0`) 0.0)
      (`KismetSystemLibrary.Delay` 1.0)
      (goto _label :!via `Reset`))))

(fn `UserConstructionScript`
  (`TimelineComponent.SetFloatCurve` (`self.タイムライン_0`) (`self.curveInstance`) "Enemy_Move"))