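; BP_Battle resolves one turn of a turn-based one-on-one battle between Hero and an enemy, using state in BP_One_v_One_GameInstance.
; Battle orders actions by NowSpd, runs attack or defence subgraphs by command number, then sets TurnEnd.
; Subgraphs call level-placed BP_Attack and BP_Defence, show text widgets timed by timelines, and display results on death.
; PowerUp and Healing adjust Hero stats, but their calling special-move logic is unconnected.
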(event `Battle`
  (bind _asbp_one_v_one_game_instance (cast `/Game/BP/BP_One_v_One_GameInstance` (`GameplayStatics.GetGameInstance`) :!pure true))
  (bind _asbp_one_v_one_game_instance_2 (cast `/Game/BP/BP_One_v_One_GameInstance` (`GameplayStatics.GetGameInstance`) :!pure true))
  (bind _asbp_one_v_one_game_instance_3 (cast `/Game/BP/BP_One_v_One_GameInstance` (`GameplayStatics.GetGameInstance`) :!pure true))
  (bind _asbp_one_v_one_game_instance_4 (cast `/Game/BP/BP_One_v_One_GameInstance` (`GameplayStatics.GetGameInstance`) :!pure true))
  (bind _asbp_one_v_one_game_instance_5 (cast `/Game/BP/BP_One_v_One_GameInstance` (`GameplayStatics.GetGameInstance`) :!pure true))
  (set `self.TurnEnd` false)
  (if (>= (`.NowSpd_30_EF77B80848F10B2EF7609FB691837994` (break `/Game/BP/BP_Character` (`/Game/BP/BP_One_v_One_GameInstance.Hero` _asbp_one_v_one_game_instance_5))) (`.NowSpd_30_EF77B80848F10B2EF7609FB691837994` (break `/Game/BP/BP_Character` (`/Game/BP/BP_One_v_One_GameInstance.Target` _asbp_one_v_one_game_instance_5))))
    (switch `int` (`.ComandNum_45_E2C8BE434526361EE38466BCF91BD0BC` (break `/Game/BP/BP_Character` (`/Game/BP/BP_One_v_One_GameInstance.Hero` (cast `/Game/BP/BP_One_v_One_GameInstance` (`GameplayStatics.GetGameInstance`) :!pure true))))
      (:`1`
        (bind _asbp_attack (`self.CastToBP_Attack`))
        (`/Game/BP/BP_Attack.Player_Atk` _asbp_attack (`/Game/BP/BP_One_v_One_GameInstance.Hero` _asbp_one_v_one_game_instance_4) (`/Game/BP/BP_One_v_One_GameInstance.Target` _asbp_one_v_one_game_instance_4))
        (bind _returnvalue (`|CreateWidget` "/Game/UI/W_Text.W_Text_C"))
        (bind _output_get (set `self.BattleText` _returnvalue))
        (`Widget.SetVisibility` (`/Game/UI/W_Text.Enemy_playerAttack` _output_get) "Hidden")
        (`Widget.SetVisibility` (`/Game/UI/W_Text.PlayerMP_None_Text` _output_get) "Hidden")
        (`Widget.SetVisibility` (`/Game/UI/W_Text.PlayerDamage_None_Text` _output_get) "Hidden")
        (`UserWidget.AddToViewport` _output_get 0)
        (`Timeline|タイムライン_2` :!via `PlayFromStart`
          (:`Finished`
            (if (`.Dead_32_2DD09B514FB38163D3DCB285D46251D5` (break `/Game/BP/BP_Character` (`/Game/BP/BP_One_v_One_GameInstance.Target` (cast `/Game/BP/BP_One_v_One_GameInstance` (`GameplayStatics.GetGameInstance`) :!pure true))))
              (`Widget.RemoveFromParent` (`self.BattleText`))
              (bind _returnvalue_2 (`|CreateWidget` "/Game/UI/W_TestResult.W_TestResult_C"))
              (bind _output_get_2 (set `self.ResultText` _returnvalue_2))
              (`Widget.SetVisibility` (`/Game/UI/W_TestResult.LoseText` _output_get_2) "Hidden")
              (`UserWidget.AddToViewport` _output_get_2 0)
              (else
                (`Widget.RemoveFromParent` (`self.BattleText`) :!label _label)
                (switch `int` (`.ComandNum_45_E2C8BE434526361EE38466BCF91BD0BC` (break `/Game/BP/BP_Character` (`/Game/BP/BP_One_v_One_GameInstance.Target` (cast `/Game/BP/BP_One_v_One_GameInstance` (`GameplayStatics.GetGameInstance`) :!pure true))))
                  (:`0`
                    (bind _asbp_attack_2 (`self.CastToBP_Attack`))
                    (`/Game/BP/BP_Attack.Enemy_Atk` _asbp_attack_2 (`/Game/BP/BP_One_v_One_GameInstance.Target` _asbp_one_v_one_game_instance) (`/Game/BP/BP_One_v_One_GameInstance.Hero` _asbp_one_v_one_game_instance))
                    (bind _returnvalue_3 (`|CreateWidget` "/Game/UI/W_Text.W_Text_C"))
                    (bind _output_get_3 (set `self.BattleText` _returnvalue_3))
                    (`Widget.SetVisibility` (`/Game/UI/W_Text.PlayerMP_None_Text` _output_get_3) "Hidden")
                    (`Widget.SetVisibility` (`/Game/UI/W_Text.Player_enemyAttack` _output_get_3) "Hidden")
                    (`Widget.SetVisibility` (`/Game/UI/W_Text.PlayerDamage_None_Text` _output_get_3) "Hidden")
                    (`UserWidget.AddToViewport` _output_get_3 0)
                    (`Timeline|タイムライン_3` :!via `PlayFromStart`
                      (:`Finished`
                        (if (`.Dead_32_2DD09B514FB38163D3DCB285D46251D5` (break `/Game/BP/BP_Character` (`/Game/BP/BP_One_v_One_GameInstance.Hero` (cast `/Game/BP/BP_One_v_One_GameInstance` (`GameplayStatics.GetGameInstance`) :!pure true))))
                          (`Widget.RemoveFromParent` (`self.BattleText`))
                          (bind _returnvalue_4 (`|CreateWidget` "/Game/UI/W_TestResult.W_TestResult_C"))
                          (bind _output_get_4 (set `self.ResultText` _returnvalue_4))
                          (`Widget.SetVisibility` (`/Game/UI/W_TestResult.WinText` _output_get_4) "Visible")
                          (`UserWidget.AddToViewport` _output_get_4 0)
                          (else
                            (`Widget.RemoveFromParent` (`self.BattleText`)))))))))))))
      (:`4`
        (bind _asbp_defence (`self.CastToBP_Defence`))
        (`/Game/BP/BP_Defence.Player_Def` _asbp_defence (`/Game/BP/BP_One_v_One_GameInstance.Hero` (cast `/Game/BP/BP_One_v_One_GameInstance` (`GameplayStatics.GetGameInstance`) :!pure true)))
        (bind _returnvalue_5 (`|CreateWidget` "/Game/UI/W_Text.W_Text_C"))
        (bind _output_get_5 (set `self.BattleText` _returnvalue_5))
        (`Widget.SetVisibility` (`/Game/UI/W_Text.Player_enemyAttack` _output_get_5) "Hidden")
        (`Widget.SetVisibility` (`/Game/UI/W_Text.PlayerMP_None_Text` _output_get_5) "Hidden")
        (`Widget.SetVisibility` (`/Game/UI/W_Text.PlayerDamage_None_Text` _output_get_5) "Hidden")
        (`Widget.SetVisibility` (`/Game/UI/W_Text.Enemy_playerAttack` _output_get_5) "Hidden")
        (`UserWidget.AddToViewport` _output_get_5 0)
        (`Timeline|タイムライン_4` :!via `PlayFromStart`
          (:`Finished`
            (goto _label)))))
    (set `self.TurnEnd` true)
    (else
      (if (== (`.ComandNum_45_E2C8BE434526361EE38466BCF91BD0BC` (break `/Game/BP/BP_Character` (`/Game/BP/BP_One_v_One_GameInstance.Hero` (cast `/Game/BP/BP_One_v_One_GameInstance` (`GameplayStatics.GetGameInstance`) :!pure true)))) 4)
        (bind _asbp_defence_2 (`self.CastToBP_Defence`))
        (`/Game/BP/BP_Defence.Player_Def` _asbp_defence_2 (`/Game/BP/BP_One_v_One_GameInstance.Hero` (cast `/Game/BP/BP_One_v_One_GameInstance` (`GameplayStatics.GetGameInstance`) :!pure true)))
        (bind _returnvalue_6 (`|CreateWidget` "/Game/UI/W_Text.W_Text_C"))
        (bind _output_get_6 (set `self.BattleText` _returnvalue_6))
        (`Widget.SetVisibility` (`/Game/UI/W_Text.PlayerMP_None_Text` _output_get_6) "Hidden")
        (`Widget.SetVisibility` (`/Game/UI/W_Text.Player_enemyAttack` _output_get_6) "Hidden")
        (`Widget.SetVisibility` (`/Game/UI/W_Text.PlayerDamage_None_Text` _output_get_6) "Hidden")
        (`Widget.SetVisibility` (`/Game/UI/W_Text.Enemy_playerAttack` _output_get_6) "Hidden")
        (`UserWidget.AddToViewport` _output_get_6 0)
        (`Timeline|タイムライン_7` :!via `PlayFromStart`
          (:`Finished`
            (`Widget.RemoveFromParent` (`self.BattleText`)))))
      (switch `int` (`.ComandNum_45_E2C8BE434526361EE38466BCF91BD0BC` (break `/Game/BP/BP_Character` (`/Game/BP/BP_One_v_One_GameInstance.Target` (cast `/Game/BP/BP_One_v_One_GameInstance` (`GameplayStatics.GetGameInstance`) :!pure true))))
        (:`0`
          (bind _asbp_attack_3 (`self.CastToBP_Attack`))
          (`/Game/BP/BP_Attack.Enemy_Atk` _asbp_attack_3 (`/Game/BP/BP_One_v_One_GameInstance.Enemy_A` _asbp_one_v_one_game_instance_2) (`/Game/BP/BP_One_v_One_GameInstance.Hero` _asbp_one_v_one_game_instance_2))
          (bind _returnvalue_7 (`|CreateWidget` "/Game/UI/W_Text.W_Text_C"))
          (bind _output_get_7 (set `self.BattleText` _returnvalue_7))
          (`Widget.SetVisibility` (`/Game/UI/W_Text.PlayerMP_None_Text` _output_get_7) "Hidden")
          (`Widget.SetVisibility` (`/Game/UI/W_Text.Player_enemyAttack` _output_get_7) "Hidden")
          (`Widget.SetVisibility` (`/Game/UI/W_Text.PlayerDamage_None_Text` _output_get_7) "Hidden")
          (`UserWidget.AddToViewport` _output_get_7 0)
          (`Timeline|タイムライン_5` :!via `PlayFromStart`
            (:`Finished`
              (if (`.Dead_32_2DD09B514FB38163D3DCB285D46251D5` (break `/Game/BP/BP_Character` (`/Game/BP/BP_One_v_One_GameInstance.Hero` (cast `/Game/BP/BP_One_v_One_GameInstance` (`GameplayStatics.GetGameInstance`) :!pure true))))
                (`Widget.RemoveFromParent` (`self.BattleText`))
                (bind _returnvalue_8 (`|CreateWidget` "/Game/UI/W_TestResult.W_TestResult_C"))
                (bind _output_get_8 (set `self.ResultText` _returnvalue_8))
                (`Widget.SetVisibility` (`/Game/UI/W_TestResult.WinText` _output_get_8) "Visible")
                (`UserWidget.AddToViewport` _output_get_8 0)
                (else
                  (`Widget.RemoveFromParent` (`self.BattleText`))
                  (switch `int` (`.ComandNum_45_E2C8BE434526361EE38466BCF91BD0BC` (break `/Game/BP/BP_Character` (`/Game/BP/BP_One_v_One_GameInstance.Hero` (cast `/Game/BP/BP_One_v_One_GameInstance` (`GameplayStatics.GetGameInstance`) :!pure true))))
                    (:`1`
                      (bind _asbp_attack_4 (`self.CastToBP_Attack`))
                      (`/Game/BP/BP_Attack.Player_Atk` _asbp_attack_4 (`/Game/BP/BP_One_v_One_GameInstance.Hero` _asbp_one_v_one_game_instance_3) (`/Game/BP/BP_One_v_One_GameInstance.Target` _asbp_one_v_one_game_instance_3))
                      (bind _returnvalue_9 (`|CreateWidget` "/Game/UI/W_Text.W_Text_C"))
                      (bind _output_get_9 (set `self.BattleText` _returnvalue_9))
                      (`Widget.SetVisibility` (`/Game/UI/W_Text.Enemy_playerAttack` _output_get_9) "Hidden")
                      (`Widget.SetVisibility` (`/Game/UI/W_Text.PlayerMP_None_Text` _output_get_9) "Hidden")
                      (`Widget.SetVisibility` (`/Game/UI/W_Text.PlayerDamage_None_Text` _output_get_9) "Hidden")
                      (`UserWidget.AddToViewport` _output_get_9 0)
                      (`Timeline|タイムライン_6` :!via `PlayFromStart`
                        (:`Finished`
                          (if (`.Dead_32_2DD09B514FB38163D3DCB285D46251D5` (break `/Game/BP/BP_Character` (`/Game/BP/BP_One_v_One_GameInstance.Enemy_A` (cast `/Game/BP/BP_One_v_One_GameInstance` (`GameplayStatics.GetGameInstance`) :!pure true))))
                            (`Widget.RemoveFromParent` (`self.BattleText`))
                            (bind _returnvalue_10 (`|CreateWidget` "/Game/UI/W_TestResult.W_TestResult_C"))
                            (bind _output_get_10 (set `self.ResultText` _returnvalue_10))
                            (`Widget.SetVisibility` (`/Game/UI/W_TestResult.LoseText` _output_get_10) "Hidden")
                            (`UserWidget.AddToViewport` _output_get_10 0)
                            (else
                              (`Widget.RemoveFromParent` (`self.BattleText`))))))))))
              (set `self.TurnEnd` true))))))))

(event `PowerUp`
  (bind _asbp_one_v_one_game_instance (cast `/Game/BP/BP_One_v_One_GameInstance` (`GameplayStatics.GetGameInstance`) :!pure true))
  (bind _hero (`/Game/BP/BP_One_v_One_GameInstance.Hero` _asbp_one_v_one_game_instance))
  (bind ((`NowMP_26_765052624FE1436EC2219F8D360B25BA` _nowmp) (`NowAtk_41_F1C25EFB436C26403D39C7B34EE08417` _nowatk)) (break `/Game/BP/BP_Character` _hero))
  (bind ((`UseMP_25_D6C7A4654BCB880703A22593AD22B2AA` _usemp) (`AtkBuf_33_E191D23944BF193DA2C73B8A1E89D5C6` _atkbuf)) (break `/Game/BP/BP_SpecialAtk` (`|GetArrayItem` (`/Game/BP/BP_One_v_One_GameInstance.Player_Spe` _asbp_one_v_one_game_instance) 1)))
  (bind _structout (setmembers `/Game/BP/BP_Character` :`StructRef` _hero :`NowMP` (- _nowmp _usemp) :`NowAtk` (`KismetMathLibrary.FTrunc` (* _nowatk _atkbuf))))
  (set `/Game/BP/BP_One_v_One_GameInstance.Hero` _structout _asbp_one_v_one_game_instance)
  (set `/Game/BP/BP_One_v_One_GameInstance.PlayerDelayCheck` false (cast `/Game/BP/BP_One_v_One_GameInstance` (`GameplayStatics.GetGameInstance`) :!pure true)))

(event `Healing`
  (bind _asbp_one_v_one_game_instance (cast `/Game/BP/BP_One_v_One_GameInstance` (`GameplayStatics.GetGameInstance`) :!pure true))
  (bind _hero (`/Game/BP/BP_One_v_One_GameInstance.Hero` _asbp_one_v_one_game_instance))
  (bind ((`NowHP_22_7C1D8F80417BE5B3F6BAC29D355D5182` _nowhp) (`NowMP_26_765052624FE1436EC2219F8D360B25BA` _nowmp)) (break `/Game/BP/BP_Character` _hero))
  (bind ((`UseMP_25_D6C7A4654BCB880703A22593AD22B2AA` _usemp) (`Heal_14_A92F38C142DA32203FA90FA6A5E90B72` _heal)) (break `/Game/BP/BP_SpecialAtk` (`|GetArrayItem` (`/Game/BP/BP_One_v_One_GameInstance.Player_Spe` _asbp_one_v_one_game_instance) 3)))
  (bind _structout (setmembers `/Game/BP/BP_Character` :`StructRef` _hero :`NowHP` (+ _nowhp _heal) :`NowMP` (- _nowmp _usemp)))
  (set `/Game/BP/BP_One_v_One_GameInstance.Hero` _structout _asbp_one_v_one_game_instance))

(event `UseSpecial`)

(fn `UserConstructionScript`)