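; BP_Attack resolves attacks between the hero and two enemies in a turn-agnostic one-v-one combat setup.
; Player_Atk and Enemy_Atk subtract attack times a randomly varied rate from target HP, also writing a damage roll into NowAtk.
; Results go to the GameInstance's Hero, EnemyA or EnemyB structs, with enemies chosen by name ("Enemy" for damage, "EnemyA" for death).
; Dead is set from the passed-in struct's HP.
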(event `Player_Atk`
  (params (Player :type "/Game/BP/BP_Character Structure (by ref)") (TargetEnemy :type "/Game/BP/BP_Character Structure (by ref)"))
  (bind (_charactername _maxhp _nowhp _maxmp _nowmp _defultatk _nowatk _defultspd _nowspd _defultdef _nowdef _rate) (break `/Game/BP/BP_Character` Player))
  (bind (_charactername_2 _maxhp_2 _nowhp_2) (break `/Game/BP/BP_Character` TargetEnemy))
  (bind _asbp_one_v_one_game_instance (cast `/Game/BP/BP_One_v_One_GameInstance` (`GameplayStatics.GetGameInstance`) :!pure true))
  (bind _asbp_one_v_one_game_instance_2 (cast `/Game/BP/BP_One_v_One_GameInstance` (`GameplayStatics.GetGameInstance`) :!pure true))
  (bind _returnvalue (`KismetMathLibrary.FTrunc` (* _nowatk (+ _rate (`KismetMathLibrary.RandomFloatInRange` -0.2 0.2)))))
  (bind _structout (setmembers `/Game/BP/BP_Character` :`StructRef` TargetEnemy :`NowHP` (- _nowhp_2 _returnvalue) :`NowAtk` _returnvalue))
  (if (== _charactername_2 "Enemy")
    (set `/Game/BP/BP_One_v_One_GameInstance.Enemy_A` _structout _asbp_one_v_one_game_instance)
    (else
      (set `/Game/BP/BP_One_v_One_GameInstance.Enemy_B` _structout _asbp_one_v_one_game_instance)))
  (if (<= (`.NowHP_22_7C1D8F80417BE5B3F6BAC29D355D5182` (break `/Game/BP/BP_Character` TargetEnemy)) 0)
    (bind _structout_2 (setmembers `/Game/BP/BP_Character` :`StructRef` TargetEnemy :`Dead` true))
    (if (== (`.CharacterName_4_60DFF35B41F76AE7F168749DF3E39C61` (break `/Game/BP/BP_Character` TargetEnemy)) "EnemyA")
      (set `/Game/BP/BP_One_v_One_GameInstance.Enemy_A` _structout_2 _asbp_one_v_one_game_instance_2)
      (else
        (set `/Game/BP/BP_One_v_One_GameInstance.Enemy_B` _structout_2 _asbp_one_v_one_game_instance_2)))))

(event `Enemy_Atk`
  (params (Enemy :type "/Game/BP/BP_Character Structure (by ref)") (TargetPlayer :type "/Game/BP/BP_Character Structure (by ref)"))
  (bind ((`DefultAtk_37_DE7D7E7D485C0A2490AC4D9808D53C6B` _defultatk) (`NowAtk_41_F1C25EFB436C26403D39C7B34EE08417` _nowatk) (`Rate_18_A4181766412355DBC196F78EF98087E2` _rate)) (break `/Game/BP/BP_Character` Enemy))
  (bind _returnvalue (`KismetMathLibrary.FTrunc` (* _nowatk (+ _rate (`KismetMathLibrary.RandomFloatInRange` -0.2 0.2)))))
  (bind _structout (setmembers `/Game/BP/BP_Character` :`StructRef` TargetPlayer :`NowHP` (- (`.NowHP_22_7C1D8F80417BE5B3F6BAC29D355D5182` (break `/Game/BP/BP_Character` TargetPlayer)) _returnvalue) :`NowAtk` _returnvalue))
  (set `/Game/BP/BP_One_v_One_GameInstance.Hero` _structout (cast `/Game/BP/BP_One_v_One_GameInstance` (`GameplayStatics.GetGameInstance`) :!pure true))
  (if (<= (`.NowHP_22_7C1D8F80417BE5B3F6BAC29D355D5182` (break `/Game/BP/BP_Character` TargetPlayer)) 0)
    (bind _structout_2 (setmembers `/Game/BP/BP_Character` :`StructRef` TargetPlayer :`Dead` true))
    (set `/Game/BP/BP_One_v_One_GameInstance.Hero` _structout_2 (cast `/Game/BP/BP_One_v_One_GameInstance` (`GameplayStatics.GetGameInstance`) :!pure true))))

(fn `UserConstructionScript`)