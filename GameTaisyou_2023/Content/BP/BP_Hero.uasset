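; BP_Hero is the player's hero actor in a one-on-one battle, animating the attack and showing item buff effects.
; Tick shows a buff emitter while GameInstance attack or defense flags are set, and polls BP_Battle's PlayerAttack to trigger movement.
; Timelines lerp the hero to a fixed strike position, with slash sound and hit particle at a TargetPoint, then back, clearing PlayerAttack.
; The construction script assigns the movement curve.
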(event `self.ReceiveTick`
  (params (DeltaSeconds :type "Float (single-precision)"))
  (bind _p_buf (`self.P_buf`))
  (bind _asbp_one_v_one_game_instance (cast `/Game/BP/BP_One_v_One_GameInstance` (`GameplayStatics.GetGameInstance`) :!pure true))
  (if (or (`/Game/BP/BP_One_v_One_GameInstance.Item_Atc_Buf` _asbp_one_v_one_game_instance) (`/Game/BP/BP_One_v_One_GameInstance.Item_Def_Buf` _asbp_one_v_one_game_instance))
    (`/Engine/EditorBlueprintResources/StandardMacros.DoOnce` false
      (:`Completed`
        (bind _returnvalue (`GameplayStatics.SpawnEmitterAtLocation` "/Game/FX/P_Buff.P_Buff" (`self.K2_GetActorLocation`)))
        (set `self.P_buf` _returnvalue)))
    (else
      (`/Engine/EditorBlueprintResources/StandardMacros.IsValid` _p_buf
        (:`Is Valid`
          (`ActorComponent.K2_DestroyComponent` _p_buf))
        (:`Is Not Valid`
          _))))
  (bind _outactors (`GameplayStatics.GetAllActorsOfClass` "/Game/BP/BP_Battle.BP_Battle_C"))
  (bind _asbp_battle (cast `/Game/BP/BP_Battle` (`|GetArrayItem` _outactors)))
  (if (`/Game/BP/BP_Battle.PlayerAttack` _asbp_battle)
    (set `self.Soundflg` true)
    (if (`self.tstflg`)
      (`self.Attack_Move`)
      (else
        (`self.Back_Move`)
        (`KismetSystemLibrary.Delay` 2.0)
        (set `self.tstflg` true)))))

(event `self.ReceiveBeginPlay`
  (set `self.Default_Position` (`self.K2_GetActorLocation`)))

(event `Attack_Move`
  (bind (_direction _enemy_move) (`Timeline|タイムライン_0`)
    (:`Update`
      (`self.K2_SetActorLocation` (`KismetMathLibrary.VLerp` (`self.Default_Position`) (50.0 0.0 0.0) _enemy_move))
      (if (`self.Soundflg`)
        (`KismetSystemLibrary.Delay` 0.25)
        (`/Engine/EditorBlueprintResources/StandardMacros.DoOnce` false :!label _label
          (:`Completed`
            (`GameplayStatics.PlaySound2D` "/Game/SE/Slash.Slash")
            (set `self.Soundflg` false)))))
    (:`Finished`
      (bind _outactors (`GameplayStatics.GetAllActorsOfClass` "/Script/Engine.TargetPoint"))
      (bind _astarget_point (cast `TargetPoint` (`|GetArrayItem` _outactors)))
      (`GameplayStatics.SpawnEmitterAtLocation` "/Game/FX/P_Hit.P_Hit" (`self.K2_GetActorLocation` _astarget_point))
      (set `self.tstflg` false))))

(event `Back_Move`
  (bind (_direction _enemy_move) (`Timeline|タイムライン_1`)
    (:`Update`
      (`self.K2_SetActorLocation` (`KismetMathLibrary.VLerp` (50.0 0.0 0.0) (`self.Default_Position`) _enemy_move)))
    (:`Finished`
      (set `/Game/BP/BP_Battle.PlayerAttack` false (stale `self.ReceiveTick` _asbp_battle))
      (`TimelineComponent.SetNewTime` (`self.タイムライン_1`) 0.0)
      (`TimelineComponent.SetNewTime` (`self.タイムライン_0`) 0.0)
      (`KismetSystemLibrary.Delay` 1.0)
      (goto _label :!via `Reset`))))

(fn `UserConstructionScript`
  (`TimelineComponent.SetFloatCurve` (`self.タイムライン_0`) (`self.curveInstance`) "Enemy_Move"))