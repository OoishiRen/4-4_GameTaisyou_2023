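; BP_P2 is an enemy combatant in a one-on-one battle that performs an attack movement.
; Tick polls BP_Battle's EnemyAttack flag and plays a timeline that lerps the actor from the GameInstance's EnemyPosition toward a fixed point.
; Timeline event tracks play the slash sound and spawn a hit particle at PlayerPosition.
; On finish, the timeline time is reset and EnemyAttack is cleared.
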(event `self.ReceiveTick`
  (params (DeltaSeconds :type "Float (single-precision)"))
  (bind _outactors (`GameplayStatics.GetAllActorsOfClass` "/Game/BP/BP_Battle.BP_Battle_C"))
  (bind _asbp_battle (cast `/Game/BP/BP_Battle` (`|GetArrayItem` _outactors)))
  (if (`/Game/BP/BP_Battle.EnemyAttack` _asbp_battle)
    (bind (_direction _move) (`Timeline|Enemy_Move`)
      (:`Update`
        (bind _asbp_one_v_one_game_instance (cast `/Game/BP/BP_One_v_One_GameInstance` (`GameplayStatics.GetGameInstance`)))
        (`self.K2_SetActorLocation` (`KismetMathLibrary.VLerp` (`/Game/BP/BP_One_v_One_GameInstance.EnemyPosition` _asbp_one_v_one_game_instance) (50.0 0.0 0.0) _move)))
      (:`Finished`
        (`TimelineComponent.SetNewTime` (`self.Enemy_Move`) 0.0)
        (bind _outactors_2 (`GameplayStatics.GetAllActorsOfClass` "/Game/BP/BP_Battle.BP_Battle_C"))
        (bind _asbp_battle_2 (cast `/Game/BP/BP_Battle` (`|GetArrayItem` _outactors_2)))
        (set `/Game/BP/BP_Battle.EnemyAttack` false _asbp_battle_2))
      (:`SE`
        (`GameplayStatics.PlaySound2D` "/Game/SE/Slash.Slash"))
      (:`Efect`
        (bind _asbp_one_v_one_game_instance_2 (cast `/Game/BP/BP_One_v_One_GameInstance` (`GameplayStatics.GetGameInstance`)))
        (`GameplayStatics.SpawnEmitterAtLocation` "/Game/FX/P_Hit.P_Hit" (`/Game/BP/BP_One_v_One_GameInstance.PlayerPosition` _asbp_one_v_one_game_instance_2))))))

(fn `UserConstructionScript`)