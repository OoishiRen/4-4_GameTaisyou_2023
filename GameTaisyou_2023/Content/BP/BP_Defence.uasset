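; BP_Defence resolves an enemy attack on the player through the Player_Def event, apparently for a one-on-one battle.
; Damage is enemy attack times a randomly varied rate, minus player defence.
; Above 1, NowHP drops and Damage receives the same HP-minus-damage expression; otherwise only Damage becomes 1.
; It writes the character struct to the GameInstance's Hero, flagging Dead when NowHP is zero or below.
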(event `Player_Def`
  (params (Enemy :type "/Game/BP/BP_Character Structure (by ref)") (TaegetPlayer :type "/Game/BP/BP_Character Structure (by ref)"))
  (bind ((`NowHP_22_7C1D8F80417BE5B3F6BAC29D355D5182` _nowhp) (`DefultAtk_37_DE7D7E7D485C0A2490AC4D9808D53C6B` _defultatk) (`NowAtk_41_F1C25EFB436C26403D39C7B34EE08417` _nowatk) (`DefultDef_40_78FEE96843F94181956F6B9664E57C2A` _defultdef) (`NowDef_42_7491192F427A3681A29158AE6392073B` _nowdef)) (break `/Game/BP/BP_Character` TaegetPlayer))
  (bind ((`DefultAtk_37_DE7D7E7D485C0A2490AC4D9808D53C6B` _defultatk_2) (`NowAtk_41_F1C25EFB436C26403D39C7B34EE08417` _nowatk_2) (`DefultDef_40_78FEE96843F94181956F6B9664E57C2A` _defultdef_2) (`NowDef_42_7491192F427A3681A29158AE6392073B` _nowdef_2) (`Rate_18_A4181766412355DBC196F78EF98087E2` _rate)) (break `/Game/BP/BP_Character` Enemy))
  (bind _asbp_one_v_one_game_instance (cast `/Game/BP/BP_One_v_One_GameInstance` (`GameplayStatics.GetGameInstance`) :!pure true))
  (bind _returnvalue (- (`KismetMathLibrary.FTrunc` (* _nowatk_2 (+ _rate (`KismetMathLibrary.RandomFloatInRange` -0.2 0.2)))) _nowdef))
  (bind _returnvalue_2 (- _nowhp _returnvalue))
  (if (> _returnvalue 1)
    (bind _structout (setmembers `/Game/BP/BP_Character` :`StructRef` TaegetPlayer :`NowHP` _returnvalue_2 :`Damage` _returnvalue_2)) ; プレイヤーの情報
    (set `/Game/BP/BP_One_v_One_GameInstance.Hero` _structout _asbp_one_v_one_game_instance)
    (else
      (bind _structout_2 (setmembers `/Game/BP/BP_Character` :`StructRef` TaegetPlayer :`Damage` 1)) ; プレイヤーの情報
      (set `/Game/BP/BP_One_v_One_GameInstance.Hero` _structout_2 _asbp_one_v_one_game_instance)))
  (if (<= (`.NowHP_22_7C1D8F80417BE5B3F6BAC29D355D5182` (break `/Game/BP/BP_Character` TaegetPlayer)) 0)
    (bind _structout_3 (setmembers `/Game/BP/BP_Character` :`StructRef` TaegetPlayer :`Dead` true)) ; プレイヤーの情報
    (set `/Game/BP/BP_One_v_One_GameInstance.Hero` _structout_3 (cast `/Game/BP/BP_One_v_One_GameInstance` (`GameplayStatics.GetGameInstance`) :!pure true))))

(fn `UserConstructionScript`)