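; BP_Special resolves special skills in a turn-based battle for the player and two enemy types.
; Each Use_Special event switches on skill number to cast flame, charge, boosted strikes or, for player and second enemy, healing.
; It checks and spends MP using GameInstance skill tables, writing updated character structs back there.
; Strikes raise attack, then delegate to BP_Attack; charge multiplies attack unless BP_Battle's buff flag is set.
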(event `Enemy1_Use_Special`
  (params (SpecialNum :type Integer) (TargetPlayer :type "/Game/BP/BP_Character Structure") (Enemy :type "/Game/BP/BP_Character Structure"))
  (bind ((`NowMP_26_765052624FE1436EC2219F8D360B25BA` _nowmp) (`NowAtk_41_F1C25EFB436C26403D39C7B34EE08417` _nowatk)) (break `/Game/BP/BP_Character` Enemy))
  (bind ((`NowHP_22_7C1D8F80417BE5B3F6BAC29D355D5182` _nowhp)) (break `/Game/BP/BP_Character` TargetPlayer))
  (bind ((`NowMP_26_765052624FE1436EC2219F8D360B25BA` _nowmp_2)) (break `/Game/BP/BP_Character` Enemy))
  (bind ((`NowMP_26_765052624FE1436EC2219F8D360B25BA` _nowmp_3) (`NowAtk_41_F1C25EFB436C26403D39C7B34EE08417` _nowatk_2)) (break `/Game/BP/BP_Character` Enemy))
  (bind _asbp_one_v_one_game_instance (`self.Cast_To_GameInstance`))
  (bind _asbp_one_v_one_game_instance_2 (`self.Cast_To_GameInstance`))
  (bind _asbp_one_v_one_game_instance_3 (`self.Cast_To_GameInstance`))
  (bind ((`UseMP_25_D6C7A4654BCB880703A22593AD22B2AA` _usemp) (`Atk_5_5004DF4447DE3C6063662EBC66F977F8` _atk)) (break `/Game/BP/BP_SpecialAtk` (`|GetArrayItem` (`/Game/BP/BP_One_v_One_GameInstance.Enemy_Spe` _asbp_one_v_one_game_instance_2) (`/Game/BP/BP_One_v_One_GameInstance.Enemy_Special_Command` _asbp_one_v_one_game_instance_2))))
  (bind ((`UseMP_25_D6C7A4654BCB880703A22593AD22B2AA` _usemp_2) (`Atk_5_5004DF4447DE3C6063662EBC66F977F8` _atk_2)) (break `/Game/BP/BP_SpecialAtk` (`|GetArrayItem` (`/Game/BP/BP_One_v_One_GameInstance.Enemy_Spe` _asbp_one_v_one_game_instance_3) (`/Game/BP/BP_One_v_One_GameInstance.Enemy_Special_Command` _asbp_one_v_one_game_instance_3))))
  (bind ((`UseMP_25_D6C7A4654BCB880703A22593AD22B2AA` _usemp_3) (`Atk_5_5004DF4447DE3C6063662EBC66F977F8` _atk_3)) (break `/Game/BP/BP_SpecialAtk` (`|GetArrayItem` (`/Game/BP/BP_One_v_One_GameInstance.Enemy_Spe` _asbp_one_v_one_game_instance) (`/Game/BP/BP_One_v_One_GameInstance.Enemy_Special_Command` _asbp_one_v_one_game_instance))))
  (bind _output_get (set `/Game/BP/BP_One_v_One_GameInstance.Enemy_Special_Command` SpecialNum (`self.Cast_To_GameInstance`)))
  (switch `int` _output_get
    (:`0`
      (if (>= _nowmp_2 _usemp_2)
        (set `/Game/BP/BP_One_v_One_GameInstance.Enemy_MP` false (`self.Cast_To_GameInstance`))
        (bind _structout (setmembers `/Game/BP/BP_Character` :`StructRef` TargetPlayer :`NowHP` (- _nowhp _atk_2) :`Damage` _atk_2)) ; プレイヤーの情報
        (set `/Game/BP/BP_One_v_One_GameInstance.Hero` _structout (`self.Cast_To_GameInstance`))
        (bind _structout_2 (setmembers `/Game/BP/BP_Character` :`StructRef` Enemy :`NowMP` (- _nowmp_2 _usemp_2))) ; 敵の情報
        (set `/Game/BP/BP_One_v_One_GameInstance.Target` _structout_2 (`self.Cast_To_GameInstance`))
        (if (<= _nowhp 0)
          (bind _structout_3 (setmembers `/Game/BP/BP_Character` :`StructRef` TargetPlayer :`Dead` true)) ; プレイヤーの情報
          (set `/Game/BP/BP_One_v_One_GameInstance.Hero` _structout_3 (`self.Cast_To_GameInstance`)))
        (else
          (set `/Game/BP/BP_One_v_One_GameInstance.Enemy_MP` true (`self.Cast_To_GameInstance`)))))
    (:`1`
      (bind _outactors (`GameplayStatics.GetAllActorsOfClass` "/Game/BP/BP_Battle.BP_Battle_C"))
      (bind _asbp_battle (cast `/Game/BP/BP_Battle` (`|GetArrayItem` _outactors)))
      (`self.Enemy1_Charge` (`/Game/BP/BP_Battle.Enemy_Special_Atc_Buf` _asbp_battle) Enemy) ; 「ためる」発動時処理
    )
    (:`2`
      (if (>= _nowmp_3 _usemp_3)
        (set `/Game/BP/BP_One_v_One_GameInstance.Enemy_MP` false (`self.Cast_To_GameInstance`))
        (bind _structout_4 (setmembers `/Game/BP/BP_Character` :`StructRef` Enemy :`NowMP` (- _nowmp_3 _usemp_3) :`NowAtk` (+ _nowatk_2 _atk_3))) ; 敵の情報
        (set `/Game/BP/BP_One_v_One_GameInstance.Target` _structout_4 (`self.Cast_To_GameInstance`))
        (bind _outactors_2 (`GameplayStatics.GetAllActorsOfClass` "/Game/BP/BP_Attack.BP_Attack_C"))
        (bind _asbp_attack (cast `/Game/BP/BP_Attack` (`|GetArrayItem` _outactors_2)))
        (`/Game/BP/BP_Attack.Enemy_Atk` _asbp_attack Enemy TargetPlayer)
        (else
          (set `/Game/BP/BP_One_v_One_GameInstance.Enemy_MP` true (`self.Cast_To_GameInstance`)))))
    (:`3`
      (if (>= _nowmp _usemp)
        (set `/Game/BP/BP_One_v_One_GameInstance.Enemy_MP` false (`self.Cast_To_GameInstance`))
        (bind _structout_5 (setmembers `/Game/BP/BP_Character` :`StructRef` Enemy :`NowMP` (- _nowmp _usemp) :`NowAtk` (+ _nowatk _atk))) ; 敵の情報
        (set `/Game/BP/BP_One_v_One_GameInstance.Target` _structout_5 (`self.Cast_To_GameInstance`))
        (bind _outactors_3 (`GameplayStatics.GetAllActorsOfClass` "/Game/BP/BP_Attack.BP_Attack_C"))
        (bind _asbp_attack_2 (cast `/Game/BP/BP_Attack` (`|GetArrayItem` _outactors_3)))
        (`/Game/BP/BP_Attack.Enemy_Atk` _asbp_attack_2 Enemy TargetPlayer)
        (else
          (set `/Game/BP/BP_One_v_One_GameInstance.Enemy_MP` true (`self.Cast_To_GameInstance`)))))))

(event `Player_Use_Special`
  (params (SpecialNum :type Integer) (TargetEnemy :type "/Game/BP/BP_Character Structure") (Player :type "/Game/BP/BP_Character Structure"))
  (bind ((`MaxHP_19_CA06E95947FC7016BD1C69AC8C5500BD` _maxhp) (`NowHP_22_7C1D8F80417BE5B3F6BAC29D355D5182` _nowhp)) (break `/Game/BP/BP_Character` Player))
  (bind ((`NowMP_26_765052624FE1436EC2219F8D360B25BA` _nowmp) (`NowAtk_41_F1C25EFB436C26403D39C7B34EE08417` _nowatk)) (break `/Game/BP/BP_Character` Player))
  (bind ((`NowHP_22_7C1D8F80417BE5B3F6BAC29D355D5182` _nowhp_2)) (break `/Game/BP/BP_Character` TargetEnemy))
  (bind ((`NowMP_26_765052624FE1436EC2219F8D360B25BA` _nowmp_2)) (break `/Game/BP/BP_Character` Player))
  (bind ((`NowMP_26_765052624FE1436EC2219F8D360B25BA` _nowmp_3)) (break `/Game/BP/BP_Character` Player))
  (bind ((`MaxHP_19_CA06E95947FC7016BD1C69AC8C5500BD` _maxhp_2) (`NowHP_22_7C1D8F80417BE5B3F6BAC29D355D5182` _nowhp_3)) (break `/Game/BP/BP_Character` Player))
  (bind ((`NowMP_26_765052624FE1436EC2219F8D360B25BA` _nowmp_4) (`NowAtk_41_F1C25EFB436C26403D39C7B34EE08417` _nowatk_2)) (break `/Game/BP/BP_Character` Player))
  (bind _asbp_one_v_one_game_instance (`self.Cast_To_GameInstance`))
  (bind _asbp_one_v_one_game_instance_2 (`self.Cast_To_GameInstance`))
  (bind _asbp_one_v_one_game_instance_3 (`self.Cast_To_GameInstance`))
  (bind _asbp_one_v_one_game_instance_4 (`self.Cast_To_GameInstance`))
  (bind ((`UseMP_25_D6C7A4654BCB880703A22593AD22B2AA` _usemp) (`Atk_5_5004DF4447DE3C6063662EBC66F977F8` _atk)) (break `/Game/BP/BP_SpecialAtk` (`|GetArrayItem` (`/Game/BP/BP_One_v_One_GameInstance.Player_Spe` (`self.Cast_To_GameInstance`)) (`self.Player_SpecialNum`))))
  (bind ((`UseMP_25_D6C7A4654BCB880703A22593AD22B2AA` _usemp_2) (`Atk_5_5004DF4447DE3C6063662EBC66F977F8` _atk_2)) (break `/Game/BP/BP_SpecialAtk` (`|GetArrayItem` (`/Game/BP/BP_One_v_One_GameInstance.Player_Spe` (`self.Cast_To_GameInstance`)) (`self.Player_SpecialNum`))))
  (bind ((`UseMP_25_D6C7A4654BCB880703A22593AD22B2AA` _usemp_3) (`Heal_14_A92F38C142DA32203FA90FA6A5E90B72` _heal)) (break `/Game/BP/BP_SpecialAtk` (`|GetArrayItem` (`/Game/BP/BP_One_v_One_GameInstance.Player_Spe` (`self.Cast_To_GameInstance`)) (`self.Player_SpecialNum`))))
  (bind ((`UseMP_25_D6C7A4654BCB880703A22593AD22B2AA` _usemp_4) (`Atk_5_5004DF4447DE3C6063662EBC66F977F8` _atk_3)) (break `/Game/BP/BP_SpecialAtk` (`|GetArrayItem` (`/Game/BP/BP_One_v_One_GameInstance.Player_Spe` (`self.Cast_To_GameInstance`)) (`self.Player_SpecialNum`))))
  (bind _returnvalue (- _nowmp_3 _usemp_3))
  (bind _returnvalue_2 (+ _nowhp_3 _heal))
  (bind _output_get (set `self.Player_SpecialNum` SpecialNum))
  (switch `int` _output_get
    (:`0`
      (if (>= _nowmp_2 _usemp_2)
        (bind _structout (setmembers `/Game/BP/BP_Character` :`StructRef` TargetEnemy :`NowHP` (- _nowhp_2 _atk_2) :`Damage` _atk_2)) ; 敵の情報
        (set `/Game/BP/BP_One_v_One_GameInstance.Target` _structout (`self.Cast_To_GameInstance`))
        (if (== (`.CharacterName_4_60DFF35B41F76AE7F168749DF3E39C61` (break `/Game/BP/BP_Character` TargetEnemy)) "Enemy")
          (set `/Game/BP/BP_One_v_One_GameInstance.Enemy_A` _structout _asbp_one_v_one_game_instance_2)
          (else
            (set `/Game/BP/BP_One_v_One_GameInstance.Enemy_B` _structout _asbp_one_v_one_game_instance_2)))
        (bind _structout_2 (setmembers `/Game/BP/BP_Character` :`StructRef` Player :`NowMP` (- _nowmp_2 _usemp_2))) ; プレイヤーの情報
        (set `/Game/BP/BP_One_v_One_GameInstance.Hero` _structout_2 (`self.Cast_To_GameInstance`))
        (if (<= _nowhp_2 0)
          (bind _structout_3 (setmembers `/Game/BP/BP_Character` :`StructRef` TargetEnemy :`Dead` true)) ; 敵の情報
          (set `/Game/BP/BP_One_v_One_GameInstance.Target` _structout_3 _asbp_one_v_one_game_instance_3)
          (if (== (`.CharacterName_4_60DFF35B41F76AE7F168749DF3E39C61` (break `/Game/BP/BP_Character` TargetEnemy)) "Enemy")
            (set `/Game/BP/BP_One_v_One_GameInstance.Enemy_A` _structout_3 _asbp_one_v_one_game_instance_3)
            (else
              (set `/Game/BP/BP_One_v_One_GameInstance.Enemy_B` _structout_3 _asbp_one_v_one_game_instance_3))))))
    (:`1`
      (bind _outactors (`GameplayStatics.GetAllActorsOfClass` "/Game/BP/BP_Battle.BP_Battle_C"))
      (bind _asbp_battle (cast `/Game/BP/BP_Battle` (`|GetArrayItem` _outactors)))
      (`self.Charge` (`/Game/BP/BP_Battle.Player_Special_Atc_buf` _asbp_battle) Player))
    (:`2`
      (if (>= _nowmp _usemp)
        (bind _structout_4 (setmembers `/Game/BP/BP_Character` :`StructRef` Player :`NowMP` (- _nowmp _usemp) :`NowAtk` (+ _nowatk _atk))) ; プレイヤーの情報
        (set `/Game/BP/BP_One_v_One_GameInstance.Hero` _structout_4 (`self.Cast_To_GameInstance`))
        (bind _outactors_2 (`GameplayStatics.GetAllActorsOfClass` "/Game/BP/BP_Attack.BP_Attack_C"))
        (bind _asbp_attack (cast `/Game/BP/BP_Attack` (`|GetArrayItem` _outactors_2)))
        (`/Game/BP/BP_Attack.Player_Atk` _asbp_attack Player TargetEnemy)))
    (:`3`
      (if (== _maxhp _nowhp)
        (set `/Game/BP/BP_One_v_One_GameInstance.Player_HP_Max` true _asbp_one_v_one_game_instance)
        (else
          (set `/Game/BP/BP_One_v_One_GameInstance.Player_HP_Max` false _asbp_one_v_one_game_instance)
          (if (>= _nowmp_3 _usemp_3)
            (if (>= _returnvalue_2 _maxhp_2)
              (bind _structout_5 (setmembers `/Game/BP/BP_Character` :`StructRef` Player :`NowHP` _maxhp_2 :`NowMP` _returnvalue)) ; プレイヤーの情報
              (set `/Game/BP/BP_One_v_One_GameInstance.Hero` _structout_5 _asbp_one_v_one_game_instance_4)
              (else
                (bind _structout_6 (setmembers `/Game/BP/BP_Character` :`StructRef` Player :`NowHP` _returnvalue_2 :`NowMP` _returnvalue)) ; プレイヤーの情報
                (set `/Game/BP/BP_One_v_One_GameInstance.Hero` _structout_6 _asbp_one_v_one_game_instance_4)))))))
    (:`4`
      (if (>= _nowmp_4 _usemp_4)
        (bind _structout_7 (setmembers `/Game/BP/BP_Character` :`StructRef` Player :`NowMP` (- _nowmp_4 _usemp_4) :`NowAtk` (+ _nowatk_2 _atk_3))) ; プレイヤーの情報
        (set `/Game/BP/BP_One_v_One_GameInstance.Hero` _structout_7 (`self.Cast_To_GameInstance`))
        (bind _outactors_3 (`GameplayStatics.GetAllActorsOfClass` "/Game/BP/BP_Attack.BP_Attack_C"))
        (bind _asbp_attack_2 (cast `/Game/BP/BP_Attack` (`|GetArrayItem` _outactors_3)))
        (`/Game/BP/BP_Attack.Player_Atk` _asbp_attack_2 Player TargetEnemy)))))

(event `Enemy2_Use_Special`
  (params (SpecialNum :type Integer) (TargetPlayer :type "/Game/BP/BP_Character Structure") (Enemy :type "/Game/BP/BP_Character Structure"))
  (bind ((`MaxHP_19_CA06E95947FC7016BD1C69AC8C5500BD` _maxhp) (`NowHP_22_7C1D8F80417BE5B3F6BAC29D355D5182` _nowhp)) (break `/Game/BP/BP_Character` Enemy))
  (bind ((`NowMP_26_765052624FE1436EC2219F8D360B25BA` _nowmp) (`NowAtk_41_F1C25EFB436C26403D39C7B34EE08417` _nowatk)) (break `/Game/BP/BP_Character` Enemy))
  (bind ((`NowMP_26_765052624FE1436EC2219F8D360B25BA` _nowmp_2)) (break `/Game/BP/BP_Character` Enemy))
  (bind ((`NowHP_22_7C1D8F80417BE5B3F6BAC29D355D5182` _nowhp_2)) (break `/Game/BP/BP_Character` TargetPlayer))
  (bind ((`NowMP_26_765052624FE1436EC2219F8D360B25BA` _nowmp_3)) (break `/Game/BP/BP_Character` Enemy))
  (bind ((`NowMP_26_765052624FE1436EC2219F8D360B25BA` _nowmp_4) (`NowAtk_41_F1C25EFB436C26403D39C7B34EE08417` _nowatk_2)) (break `/Game/BP/BP_Character` Enemy))
  (bind ((`MaxHP_19_CA06E95947FC7016BD1C69AC8C5500BD` _maxhp_2)) (break `/Game/BP/BP_Character` Enemy))
  (bind _asbp_one_v_one_game_instance (`self.Cast_To_GameInstance`))
  (bind _asbp_one_v_one_game_instance_2 (`self.Cast_To_GameInstance`))
  (bind _asbp_one_v_one_game_instance_3 (`self.Cast_To_GameInstance`))
  (bind _asbp_one_v_one_game_instance_4 (`self.Cast_To_GameInstance`))
  (bind _asbp_one_v_one_game_instance_5 (`self.Cast_To_GameInstance`))
  (bind _asbp_one_v_one_game_instance_6 (`self.Cast_To_GameInstance`))
  (bind ((`UseMP_25_D6C7A4654BCB880703A22593AD22B2AA` _usemp) (`Atk_5_5004DF4447DE3C6063662EBC66F977F8` _atk)) (break `/Game/BP/BP_SpecialAtk` (`|GetArrayItem` (`/Game/BP/BP_One_v_One_GameInstance.Enemy2_Spe` _asbp_one_v_one_game_instance_2) (`/Game/BP/BP_One_v_One_GameInstance.Enemy_Special_Command` _asbp_one_v_one_game_instance_2))))
  (bind ((`UseMP_25_D6C7A4654BCB880703A22593AD22B2AA` _usemp_2) (`Heal_14_A92F38C142DA32203FA90FA6A5E90B72` _heal)) (break `/Game/BP/BP_SpecialAtk` (`|GetArrayItem` (`/Game/BP/BP_One_v_One_GameInstance.Enemy2_Spe` _asbp_one_v_one_game_instance_4) (`/Game/BP/BP_One_v_One_GameInstance.Enemy_Special_Command` _asbp_one_v_one_game_instance_4))))
  (bind ((`UseMP_25_D6C7A4654BCB880703A22593AD22B2AA` _usemp_3) (`Atk_5_5004DF4447DE3C6063662EBC66F977F8` _atk_2)) (break `/Game/BP/BP_SpecialAtk` (`|GetArrayItem` (`/Game/BP/BP_One_v_One_GameInstance.Enemy2_Spe` _asbp_one_v_one_game_instance_6) (`/Game/BP/BP_One_v_One_GameInstance.Enemy_Special_Command` _asbp_one_v_one_game_instance_6))))
  (bind ((`UseMP_25_D6C7A4654BCB880703A22593AD22B2AA` _usemp_4) (`Atk_5_5004DF4447DE3C6063662EBC66F977F8` _atk_3)) (break `/Game/BP/BP_SpecialAtk` (`|GetArrayItem` (`/Game/BP/BP_One_v_One_GameInstance.Enemy2_Spe` _asbp_one_v_one_game_instance) (`/Game/BP/BP_One_v_One_GameInstance.Enemy_Special_Command` _asbp_one_v_one_game_instance))))
  (bind _returnvalue (- _nowmp_2 _usemp_2))
  (bind _returnvalue_2 (+ _heal (`.NowHP_22_7C1D8F80417BE5B3F6BAC29D355D5182` (break `/Game/BP/BP_Character` Enemy))))
  (bind _output_get (set `/Game/BP/BP_One_v_One_GameInstance.Enemy_Special_Command` SpecialNum (`self.Cast_To_GameInstance`)))
  (switch `int` _output_get
    (:`0`
      (if (>= _nowmp_3 _usemp_3)
        (set `/Game/BP/BP_One_v_One_GameInstance.Enemy_MP` false (`self.Cast_To_GameInstance`))
        (bind _structout (setmembers `/Game/BP/BP_Character` :`StructRef` TargetPlayer :`NowHP` (- _nowhp_2 _atk_2) :`Damage` _atk_2)) ; プレイヤーの情報
        (set `/Game/BP/BP_One_v_One_GameInstance.Hero` _structout (`self.Cast_To_GameInstance`))
        (bind _structout_2 (setmembers `/Game/BP/BP_Character` :`StructRef` Enemy :`NowMP` (- _nowmp_3 _usemp_3))) ; 敵の情報
        (set `/Game/BP/BP_One_v_One_GameInstance.Target` _structout_2 (`self.Cast_To_GameInstance`))
        (if (<= _nowhp_2 0)
          (bind _structout_3 (setmembers `/Game/BP/BP_Character` :`StructRef` TargetPlayer :`Dead` true)) ; プレイヤーの情報
          (set `/Game/BP/BP_One_v_One_GameInstance.Hero` _structout_3 (`self.Cast_To_GameInstance`)))
        (else
          (set `/Game/BP/BP_One_v_One_GameInstance.Enemy_MP` true (`self.Cast_To_GameInstance`)))))
    (:`1`
      (bind _outactors (`GameplayStatics.GetAllActorsOfClass` "/Game/BP/BP_Battle.BP_Battle_C"))
      (bind _asbp_battle (cast `/Game/BP/BP_Battle` (`|GetArrayItem` _outactors)))
      (`self.Enemy2_Charge` (`/Game/BP/BP_Battle.Enemy_Special_Atc_Buf` _asbp_battle) Enemy) ; 「ためる」発動時処理
    )
    (:`2`
      (if (>= _nowmp _usemp)
        (set `/Game/BP/BP_One_v_One_GameInstance.Enemy_MP` false (`self.Cast_To_GameInstance`))
        (bind _structout_4 (setmembers `/Game/BP/BP_Character` :`StructRef` Enemy :`NowMP` (- _nowmp _usemp) :`NowAtk` (+ _nowatk _atk))) ; 敵の情報
        (set `/Game/BP/BP_One_v_One_GameInstance.Target` _structout_4 (`self.Cast_To_GameInstance`))
        (bind _outactors_2 (`GameplayStatics.GetAllActorsOfClass` "/Game/BP/BP_Attack.BP_Attack_C"))
        (bind _asbp_attack (cast `/Game/BP/BP_Attack` (`|GetArrayItem` _outactors_2)))
        (`/Game/BP/BP_Attack.Enemy_Atk` _asbp_attack Enemy TargetPlayer)
        (else
          (set `/Game/BP/BP_One_v_One_GameInstance.Enemy_MP` true (`self.Cast_To_GameInstance`)))))
    (:`3`
      (if (>= _nowmp_4 _usemp_4)
        (set `/Game/BP/BP_One_v_One_GameInstance.Enemy_MP` false (`self.Cast_To_GameInstance`))
        (bind _structout_5 (setmembers `/Game/BP/BP_Character` :`StructRef` Enemy :`NowMP` (- _nowmp_4 _usemp_4) :`NowAtk` (+ _nowatk_2 _atk_3))) ; 敵の情報
        (set `/Game/BP/BP_One_v_One_GameInstance.Target` _structout_5 (`self.Cast_To_GameInstance`))
        (bind _outactors_3 (`GameplayStatics.GetAllActorsOfClass` "/Game/BP/BP_Attack.BP_Attack_C"))
        (bind _asbp_attack_2 (cast `/Game/BP/BP_Attack` (`|GetArrayItem` _outactors_3)))
        (`/Game/BP/BP_Attack.Enemy_Atk` _asbp_attack_2 Enemy TargetPlayer)
        (else
          (set `/Game/BP/BP_One_v_One_GameInstance.Enemy_MP` true (`self.Cast_To_GameInstance`)))))
    (:`4`
      (if (== _maxhp _nowhp)
        (set `/Game/BP/BP_One_v_One_GameInstance.Enemy_HP_Max` true _asbp_one_v_one_game_instance_3)
        (else
          (set `/Game/BP/BP_One_v_One_GameInstance.Enemy_HP_Max` false _asbp_one_v_one_game_instance_3)
          (if (>= _nowmp_2 _usemp_2)
            (set `/Game/BP/BP_One_v_One_GameInstance.Enemy_MP` false (`self.Cast_To_GameInstance`))
            (if (>= _returnvalue_2 _maxhp_2)
              (bind _structout_6 (setmembers `/Game/BP/BP_Character` :`StructRef` Enemy :`NowHP` _maxhp_2 :`NowMP` _returnvalue)) ; 敵の情報
              (set `/Game/BP/BP_One_v_One_GameInstance.Target` _structout_6 _asbp_one_v_one_game_instance_5)
              (else
                (bind _structout_7 (setmembers `/Game/BP/BP_Character` :`StructRef` Enemy :`NowHP` _returnvalue_2 :`NowMP` _returnvalue)) ; 敵の情報
                (set `/Game/BP/BP_One_v_One_GameInstance.Target` _structout_7 _asbp_one_v_one_game_instance_5)))
            (else
              (set `/Game/BP/BP_One_v_One_GameInstance.Enemy_MP` true (`self.Cast_To_GameInstance`)))))))))

(event `Charge`
  (params (Buf_Flg :type Boolean) (Player :type "/Game/BP/BP_Character Structure"))
  (bind ((`NowMP_26_765052624FE1436EC2219F8D360B25BA` _nowmp)) (break `/Game/BP/BP_Character` Player))
  (bind ((`UseMP_25_D6C7A4654BCB880703A22593AD22B2AA` _usemp) (`AtkBuf_33_E191D23944BF193DA2C73B8A1E89D5C6` _atkbuf)) (break `/Game/BP/BP_SpecialAtk` (`|GetArrayItem` (`/Game/BP/BP_One_v_One_GameInstance.Player_Spe` (`self.Cast_To_GameInstance`)) (`self.Player_SpecialNum`))))
  (if Buf_Flg
    _
    (elif (>= _nowmp _usemp)
      (bind _structout (setmembers `/Game/BP/BP_Character` :`StructRef` Player :`NowMP` (- _nowmp _usemp) :`NowAtk` (`KismetMathLibrary.FTrunc` (* (`.NowAtk_41_F1C25EFB436C26403D39C7B34EE08417` (break `/Game/BP/BP_Character` Player)) _atkbuf)))) ; プレイヤーの情報
      (set `/Game/BP/BP_One_v_One_GameInstance.Hero` _structout (`self.Cast_To_GameInstance`)))))

(event `Enemy1_Charge`
  (params (Buf_Flg :type Boolean) (Target :type "/Game/BP/BP_Character Structure (by ref)"))
  (bind ((`NowMP_26_765052624FE1436EC2219F8D360B25BA` _nowmp)) (break `/Game/BP/BP_Character` Target))
  (bind _asbp_one_v_one_game_instance (`self.Cast_To_GameInstance`))
  (bind ((`UseMP_25_D6C7A4654BCB880703A22593AD22B2AA` _usemp) (`AtkBuf_33_E191D23944BF193DA2C73B8A1E89D5C6` _atkbuf)) (break `/Game/BP/BP_SpecialAtk` (`|GetArrayItem` (`/Game/BP/BP_One_v_One_GameInstance.Enemy_Spe` _asbp_one_v_one_game_instance) (`/Game/BP/BP_One_v_One_GameInstance.Enemy_Special_Command` _asbp_one_v_one_game_instance))))
  (if Buf_Flg
    _
    (elif (>= _nowmp _usemp)
      (set `/Game/BP/BP_One_v_One_GameInstance.Enemy_MP` false (`self.Cast_To_GameInstance`))
      (bind _structout (setmembers `/Game/BP/BP_Character` :`StructRef` Target :`NowMP` (- _nowmp _usemp) :`NowAtk` (`KismetMathLibrary.FTrunc` (* (`.NowAtk_41_F1C25EFB436C26403D39C7B34EE08417` (break `/Game/BP/BP_Character` Target)) _atkbuf)))) ; 敵の情報
      (set `/Game/BP/BP_One_v_One_GameInstance.Target` _structout (`self.Cast_To_GameInstance`))
      (else
        (set `/Game/BP/BP_One_v_One_GameInstance.Enemy_MP` true (`self.Cast_To_GameInstance`))))))

(event `Enemy2_Charge`
  (params (Buf_Flg :type Boolean) (Target :type "/Game/BP/BP_Character Structure"))
  (bind ((`NowMP_26_765052624FE1436EC2219F8D360B25BA` _nowmp)) (break `/Game/BP/BP_Character` Target))
  (bind _asbp_one_v_one_game_instance (`self.Cast_To_GameInstance`))
  (bind ((`UseMP_25_D6C7A4654BCB880703A22593AD22B2AA` _usemp) (`AtkBuf_33_E191D23944BF193DA2C73B8A1E89D5C6` _atkbuf)) (break `/Game/BP/BP_SpecialAtk` (`|GetArrayItem` (`/Game/BP/BP_One_v_One_GameInstance.Enemy2_Spe` _asbp_one_v_one_game_instance) (`/Game/BP/BP_One_v_One_GameInstance.Enemy_Special_Command` _asbp_one_v_one_game_instance))))
  (if Buf_Flg
    _
    (elif (>= _nowmp _usemp)
      (set `/Game/BP/BP_One_v_One_GameInstance.Enemy_MP` false (`self.Cast_To_GameInstance`))
      (bind _structout (setmembers `/Game/BP/BP_Character` :`StructRef` Target :`NowMP` (- _nowmp _usemp) :`NowAtk` (`KismetMathLibrary.FTrunc` (* (`.NowAtk_41_F1C25EFB436C26403D39C7B34EE08417` (break `/Game/BP/BP_Character` Target)) _atkbuf)))) ; 敵の情報
      (set `/Game/BP/BP_One_v_One_GameInstance.Target` _structout (`self.Cast_To_GameInstance`))
      (else
        (set `/Game/BP/BP_One_v_One_GameInstance.Enemy_MP` true (`self.Cast_To_GameInstance`))))))

(fn `UserConstructionScript`)